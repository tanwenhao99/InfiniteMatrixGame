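; BP_HealthPack is a rotating health pickup for BP_Player.
; On player overlap it shows a new GreenScreenHUD widget, destroys the HealthPack component (not the actor) and adds a fixed health amount if CurrentHealth is below full, without clamping.
; An overlapping BP_Bullet is destroyed, leaving the pack intact.
; Tick yaws the component at RotateSpeed while it remains valid.
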(event OnComponentBeginOverlap(HealthPack)
  (params (OverlappedComponent :type Primitive%20Component%20Object%20Reference) (OtherActor :type Actor%20Object%20Reference) (OtherComp :type Primitive%20Component%20Object%20Reference) (OtherBodyIndex :type Integer) (bFromSweep :type Boolean) (SweepResult :type Hit%20Result%20Structure%20%28by%20ref%29))
  (bind _asbp_player (Utilities|Casting|CastToBP_Player OtherActor)
    (:then
      (bind _returnvalue (UserInterface|CreateWidget "/Game/InfiniteMatrix/UI/GreenScreenHUD.GreenScreenHUD_C"))
      (UserInterface|Viewport|AddtoViewport _returnvalue 0)
      (Components|DestroyComponent OverlappedComponent)
      (if (< (Variables|/Game/InfiniteMatrix/Blueprints/BP_Player.BP_Player_C|GetCurrentHealth _asbp_player) 1e+02)
        (Variables|/Game/InfiniteMatrix/Blueprints/BP_Player.BP_Player_C|SetCurrentHealth _asbp_player (+ 1e+01 (Variables|/Game/InfiniteMatrix/Blueprints/BP_Player.BP_Player_C|GetCurrentHealth _asbp_player)))))
    (:CastFailed
      (bind _asbp_bullet (Utilities|Casting|CastToBP_Bullet OtherActor))
      (Actor|DestroyActor _asbp_bullet))))

(event EventBeginPlay)

(event EventTick
  (params (DeltaSeconds :type Float%20%28single-precision%29))
  (bind _healthpack (Variables|Default|GetHealthPack))
  (Utilities|IsValid _healthpack
    (:Is%20Valid
      (Transformation|AddLocalRotation _healthpack (Math|Rotator|MakeRotator 0.0 0.0 (* DeltaSeconds (Variables|Default|GetRotateSpeed))) false false))))

(fn ConstructionScript)