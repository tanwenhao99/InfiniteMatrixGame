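; BP_Bomb is a spinning hazard that hurts the player on contact or can be shot for points.
; Player overlap triggers a world camera shake and red-screen widget, deducts score and health, and shows the restart screen when health equals exactly zero.
; A bullet overlap destroys the bullet and awards score to the player pawn.
; Either hit destroys only the Bomb component, which Tick rotates while valid.
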(event OnComponentBeginOverlap(Bomb)
  (params (OverlappedComponent :type Primitive%20Component%20Object%20Reference) (OtherActor :type Actor%20Object%20Reference) (OtherComp :type Primitive%20Component%20Object%20Reference) (OtherBodyIndex :type Integer) (bFromSweep :type Boolean) (SweepResult :type Hit%20Result%20Structure%20%28by%20ref%29))
  (bind _asbp_player (Utilities|Casting|CastToBP_Player OtherActor)
    (:then
      (Camera|PlayWorldCameraShake "/Game/InfiniteMatrix/Blueprints/BP_CameraShake.BP_CameraShake_C" (Transformation|GetWorldLocation OverlappedComponent) 1e+02 1e+03)
      (bind _returnvalue (UserInterface|CreateWidget "/Game/InfiniteMatrix/UI/RedScreenHUD.RedScreenHUD_C"))
      (UserInterface|Viewport|AddtoViewport _returnvalue 0)
      (Components|DestroyComponent OverlappedComponent)
      (Variables|/Game/InfiniteMatrix/Blueprints/BP_Player.BP_Player_C|SetScore _asbp_player (- (Variables|/Game/InfiniteMatrix/Blueprints/BP_Player.BP_Player_C|GetScore _asbp_player) 10))
      (bind _output_get (Variables|/Game/InfiniteMatrix/Blueprints/BP_Player.BP_Player_C|SetCurrentHealth _asbp_player (- (Variables|/Game/InfiniteMatrix/Blueprints/BP_Player.BP_Player_C|GetCurrentHealth _asbp_player) 1e+01)))
      (if (== _output_get 0.0)
        (Variables|/Game/InfiniteMatrix/Blueprints/BP_Player.BP_Player_C|SetIsDead _asbp_player true)
        (Default|DisplayRestart _asbp_player)))
    (:CastFailed
      (bind _asbp_bullet (Utilities|Casting|CastToBP_Bullet OtherActor))
      (Actor|DestroyActor _asbp_bullet)
      (bind _asbp_player_2 (Utilities|Casting|CastToBP_Player (Game|Player|GetPlayerPawn 0)))
      (Variables|/Game/InfiniteMatrix/Blueprints/BP_Player.BP_Player_C|SetScore _asbp_player_2 (+ 50 (Variables|/Game/InfiniteMatrix/Blueprints/BP_Player.BP_Player_C|GetScore _asbp_player_2)))
      (Components|DestroyComponent OverlappedComponent))))

(event EventTick
  (params (DeltaSeconds :type Float%20%28single-precision%29))
  (bind _bomb (Variables|Default|GetBomb))
  (Utilities|IsValid _bomb
    (:Is%20Valid
      (Transformation|AddLocalRotation _bomb (Math|Rotator|MakeRotator 0.0 0.0 (* DeltaSeconds (Variables|Default|GetRotateSpeed))) false false))))

(fn ConstructionScript)